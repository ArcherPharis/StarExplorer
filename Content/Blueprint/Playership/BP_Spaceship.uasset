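; Player spaceship Blueprint that balances its physics mesh around the thruster and can spawn a ship interior.
; On BeginPlay it rotates the center-of-mass-to-thruster vector into mesh space and applies its X and Y as a center of mass offset.
; The TogglePlayer input spawns a new interior level instance at the ship's transform on each press, with no toggle back.
; Unconnected leftovers would open a level or pre-spawn a hidden interior.
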(event EventBeginPlay
  (bind _returnvalue (Class|BaseSpaceship|GetShipMesh))
  (bind _returnvalue_2 (Class|BaseSpaceship|GetThrusterComponent))
  (bind _returnvalue_3 (Transformation|GetWorldLocation _returnvalue_2))
  (bind _returnvalue_4 (Physics|GetCenterOfMass _returnvalue "None"))
  (bind _returnvalue_5 (Transformation|GetWorldRotation _returnvalue))
  (bind _returnvalue_6 (Class|KismetMathLibrary|NegateRotator _returnvalue_5))
  (bind _returnvalue_7 (- _returnvalue_3 _returnvalue_4))
  (bind _returnvalue_8 (Math|Vector|RotateVector _returnvalue_7 _returnvalue_6))
  (Class|PrimitiveComponent|SetCenterOfMass (Class|BaseSpaceship|GetShipMesh) (Math|Vector|MakeVector (.x _returnvalue_8) (.y _returnvalue_8) 0.0) "None"))

(event Collision|EventActorBeginOverlap
  (params (OtherActor :type Actor%20Object%20Reference)))

(event EventTick
  (params (DeltaSeconds :type Float%20%28single-precision%29)))

(event Input|ActionEvents|InputActionTogglePlayer
  (params (Key :type Key%20Structure :default "None"))
  (:Pressed
    (Game|SpawnActorfromClass "/Game/Levels/PlayerShipInterior_LevelInstance.PlayerShipInterior_LevelInstance_C" (Transformation|GetActorTransform) "AlwaysSpawn" 0 self)))

(fn ConstructionScript)